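; Enemy spawner volume that keeps spawning BP_Enemy actors inside its SpawnBox, up to a cap on the number alive.
; With AutoStart set, BeginPlay starts a looping timer that calls SpawnEnemy every SpawnInterval.
; Each spawn picks a random point in the box, raised slightly in Z, and increments CurrentAliveCount.
; Each enemy's OnDestroyed event decrements that count, clamped to valid bounds, freeing a slot for later spawns.
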(event Custom|SpawnEnemy
  (bind _spawnbox (Variables|Default|GetSpawnBox))
  (bind _returnvalue (Components|Box|GetScaledBoxExtent _spawnbox))
  (bind _returnvalue_2 (Transformation|GetWorldLocation _spawnbox))
  (bind _returnvalue_3 (Math|Random|RandomPointinBoundingBox _returnvalue_2 _returnvalue))
  (bind (_x _y _z) (Math|Vector|BreakVector _returnvalue_3))
  (if (< (Variables|Default|GetCurrentAliveCount) (Variables|Default|GetMaxAliveCount))
    (bind _returnvalue_4 (Game|SpawnActorfromClass "/Game/AI/BP_Enemy.BP_Enemy_C" (Math|Transform|MakeTransform (Math|Vector|MakeVector _x _y (+ _z 5e+01))) "Undefined" "MultiplyWithRoot" 0 0))
    (Variables|Default|SetCurrentAliveCount (+ (Variables|Default|GetCurrentAliveCount) 1))
    (Game|BindEventtoOnDestroyed _returnvalue_4 (delegate Custom|OnEnemyDestroyed))))

(event Custom|OnEnemyDestroyed
  (params (DestroyedActor :type Actor%20Object%20Reference))
  (Variables|Default|SetCurrentAliveCount (Math|Integer|Clamp(Integer) (- (Variables|Default|GetCurrentAliveCount) 1) 0 (Variables|Default|GetMaxAliveCount))))

(event EventBeginPlay
  (if (Variables|Default|GetbAutoStart)
    (Utilities|Time|SetTimerbyEvent (delegate Custom|SpawnEnemy) (Variables|Default|GetSpawnInterval) true)))

(fn ConstructionScript)