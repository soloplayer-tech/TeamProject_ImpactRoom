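; BP_Enemy is an AI enemy with health, an on-screen health bar widget and player sensing.
; Damage reduces clamped HP and refreshes the cached WBP_EnemyHealthBar, which starts full on BeginPlay.
; The actor destroys itself at zero HP, a check that runs only while the bar reference is valid.
; PawnSensing sets the blackboard's HasSeenPlayer? flag on seeing BP_ThirdPersonCharacter, and nothing here clears it.
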(event OnSeePawn(PawnSensing)
  (params (Pawn :type Pawn%20Object%20Reference))
  (Utilities|Casting|CastToBP_ThirdPersonCharacter Pawn)
  (AI|Components|Blackboard|SetValueasBool (AI|GetBlackboard (AI|GetAIController self)) (Utilities|Name|MakeLiteralName "HasSeenPlayer?") true))

(event Custom|EnemyTakeDamage
  (params (DamageAmount :type Float%20%28double-precision%29))
  (bind _output_get (Variables|Default|SetCurrentHP (Math|Float|Clamp(Float) (- (Variables|Default|GetCurrentHP) DamageAmount) 0.0 (Variables|Default|GetMaxHP))))
  (Utilities|IsValid (Variables|Default|GetHealthBarRef)
    (:Is%20Valid
      (Default|UpdateHealthBar (Variables|Default|GetHealthBarRef) (Variables|Default|GetCurrentHP) (Variables|Default|GetMaxHP))
      (if (<= _output_get 0.0)
        (Actor|DestroyActor)))))

(event EventBeginPlay
  (Variables|Default|SetCurrentHP (Variables|Default|GetMaxHP))
  (bind _aswbp_enemy_health_bar (Utilities|Casting|CastToWBP_EnemyHealthBar (UserInterface|GetUserWidgetObject (Variables|Default|GetHealthBarWidget))))
  (bind _output_get (Variables|Default|SetHealthBarRef _aswbp_enemy_health_bar))
  (Default|UpdateHealthBar _output_get (Variables|Default|GetCurrentHP) (Variables|Default|GetMaxHP)))

(event Game|Damage|EventAnyDamage
  (params (Damage :type Float%20%28single-precision%29) (DamageType :type Damage%20Type%20Object%20Reference) (InstigatedBy :type Controller%20Object%20Reference) (DamageCauser :type Actor%20Object%20Reference))
  (CallFunction|EnemyTakeDamage Damage))

(fn ConstructionScript)