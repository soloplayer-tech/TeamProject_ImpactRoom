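; BP_Bullet is a projectile actor that flies forward and kills monsters on contact.
; Each Tick, the Translate function moves it along its forward vector by Speed scaled by world delta seconds, without sweeping.
; When it begins overlapping a BP_Monster, it destroys both the monster and itself, ignoring all other actors.
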(event EventBeginPlay)

(event Collision|EventActorBeginOverlap
  (params (OtherActor :type Actor%20Object%20Reference))
  (bind _asbp_monster (Utilities|Casting|CastToBP_Monster OtherActor))
  (Actor|DestroyActor _asbp_monster)
  (Actor|DestroyActor))

(event EventTick
  (params (DeltaSeconds :type Float%20%28single-precision%29))
  (CallFunction|Translate (Variables|Default|GetSpeed)))

(fn ConstructionScript)

(fn Translate
  (params (B :type Float%20%28double-precision%29))
  (Transformation|SetActorLocation (+ (Transformation|GetActorLocation) (* (Transformation|GetActorForwardVector) B (Utilities|Time|GetWorldDeltaSeconds))) false false))